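; Enemy spawner actor that spawns batches of a set enemy class at its own transform, starting on BeginPlay.
; After each batch it compares the ThirdPersonGameMode's EnemyCount to MaxEnemyCount and, if below the cap, spawns again after SpawnDelay.
; At the cap it switches to a self-calling check event that polls every SpawnDelay until there is room again.
; The cap is only tested after spawning, so a batch can overshoot it.
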(event `self.ReceiveBeginPlay`
  (`|ExecutionSequence`
    (:`then_0`
      (bind _asthird_person_game_mode (cast `/Game/ThirdPersonBP/Blueprints/ThirdPersonGameMode` (`GameplayStatics.GetGameMode`)))
      (set `self.GameModeRef` _asthird_person_game_mode))
    (:`then_1`
      (`self.OnSpawnEnemy` (`self.EnemyClass`) (`self.GetTransform`) (`self.EnemyAmount`)))))

(event `OnSpawnEnemy`
  (params (EnemyClass :type "Actor Class Reference") (SpawnTransform :type "Transform Structure") (EnemyAmount :type Integer))
  (bind _gamemoderef (`self.GameModeRef`))
  (for _ (range EnemyAmount)
    (`|SpawnActorFromClass` EnemyClass SpawnTransform "Undefined" "OverrideRootScale" null null))
  (if (< (`/Game/ThirdPersonBP/Blueprints/ThirdPersonGameMode.EnemyCount` _gamemoderef) (`/Game/ThirdPersonBP/Blueprints/ThirdPersonGameMode.MaxEnemyCount` _gamemoderef))
    (`KismetSystemLibrary.Delay` (`self.SpawnDelay`))
    (`self.OnSpawnEnemy` (`self.EnemyClass`) (`self.GetTransform`) (`self.EnemyAmount`))
    (else
      (`self.OnCheckEnemyCount`))))

(event `OnCheckEnemyCount`
  (bind _gamemoderef (`self.GameModeRef`))
  (`KismetSystemLibrary.Delay` (`self.SpawnDelay`))
  (if (< (`/Game/ThirdPersonBP/Blueprints/ThirdPersonGameMode.EnemyCount` _gamemoderef) (`/Game/ThirdPersonBP/Blueprints/ThirdPersonGameMode.MaxEnemyCount` _gamemoderef))
    (`self.OnSpawnEnemy` (`self.EnemyClass`) (`self.GetTransform`) (`self.EnemyAmount`))
    (else
      (`self.OnCheckEnemyCount`))))

(fn `UserConstructionScript`)