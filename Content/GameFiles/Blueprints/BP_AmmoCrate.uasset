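; BP_AmmoCrate is an interactable ammo pickup that adds a fixed amount of ammo to the player character.
; A box overlap by the player enables input on the crate and shows a pickup prompt on the player's HUD; leaving disables input and hides it.
; Pressing Interact adds the ammo, plays a pickup sound and destroys the crate.
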(event `InputAction|Interact`
  (params (Key :type "Key Structure"))
  (:`Pressed`
    (bind _asbp_player_character (cast `/Game/GameFiles/Characters/BP_PlayerCharacter` (`GameplayStatics.GetPlayerCharacter` 0)))
    (set `/Game/GameFiles/Characters/BP_PlayerCharacter.Ammo` (+ (`/Game/GameFiles/Characters/BP_PlayerCharacter.Ammo` _asbp_player_character) 60) _asbp_player_character)
    (`GameplayStatics.PlaySound2D` "/Game/GameFiles/Sounds/AmmoPickUp/A_AmmoPickUp_Cue.A_AmmoPickUp_Cue" 1.0 1.0 0.0 null null)
    (`self.K2_DestroyActor`)))

(event `self.BoxCollision.OnComponentBeginOverlap`
  (params (OverlappedComponent :type "PrimitiveComponent Object Reference") (OtherActor :type "Actor Object Reference") (OtherComp :type "PrimitiveComponent Object Reference") (OtherBodyIndex :type Integer) (bFromSweep :type Boolean) (SweepResult :type "HitResult Structure (by ref)"))
  (bind _asbp_player_character (cast `/Game/GameFiles/Characters/BP_PlayerCharacter` OtherActor))
  (`self.EnableInput` (`GameplayStatics.GetPlayerController` 0))
  (bind _headsupdisplay (`/Game/GameFiles/Characters/BP_PlayerCharacter.HeadsUpDisplay` _asbp_player_character)
    (:`then`
      (bind _interactionmessage (`/Game/GameFiles/UI/WBP_HeadsUpDisplay.InteractionMessage` _headsupdisplay))
      (`TextBlock.SetText` _interactionmessage "Press F to pick up ammo")
      (`Widget.SetVisibility` _interactionmessage "Visible"))
    (:`else`)))

(event `self.BoxCollision.OnComponentEndOverlap`
  (params (OverlappedComponent :type "PrimitiveComponent Object Reference") (OtherActor :type "Actor Object Reference") (OtherComp :type "PrimitiveComponent Object Reference") (OtherBodyIndex :type Integer))
  (bind _asbp_player_character (cast `/Game/GameFiles/Characters/BP_PlayerCharacter` OtherActor))
  (`self.DisableInput` (`GameplayStatics.GetPlayerController` 0))
  (bind _headsupdisplay (`/Game/GameFiles/Characters/BP_PlayerCharacter.HeadsUpDisplay` _asbp_player_character)
    (:`then`
      (`Widget.SetVisibility` (`/Game/GameFiles/UI/WBP_HeadsUpDisplay.InteractionMessage` _headsupdisplay) "Hidden"))
    (:`else`)))

(fn `UserConstructionScript`)