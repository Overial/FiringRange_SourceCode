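; BP_JumpingPlatform is a launch pad that flings the player character upward as a ragdoll when it enters the collision box.
; Begin overlap flags BP_PlayerCharacter as ragdolled, enables physics on its mesh and applies a mass-independent upward impulse.
; End overlap sets the character's jump Z velocity to a fixed value.
; Logic to detach and simulate the gun mesh exists but is unconnected.
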(event `self.CollisionBox.OnComponentBeginOverlap`
  (params (OverlappedComponent :type "PrimitiveComponent Object Reference") (OtherActor :type "Actor Object Reference") (OtherComp :type "PrimitiveComponent Object Reference") (OtherBodyIndex :type Integer) (bFromSweep :type Boolean) (SweepResult :type "HitResult Structure (by ref)"))
  (bind _asbp_player_character (cast `/Game/GameFiles/Characters/BP_PlayerCharacter` OtherActor))
  (set `/Game/GameFiles/Characters/BP_PlayerCharacter.IsInRagdoll?` true _asbp_player_character)
  (`|ExecutionSequence`
    (:`then_0`
      (bind _mesh (`Character.Mesh` _asbp_player_character))
      (`PrimitiveComponent.SetCollisionEnabled` _mesh "QueryAndPhysics")
      (`SkeletalMeshComponent.SetAllBodiesSimulatePhysics` _mesh true)
      (`PrimitiveComponent.SetSimulatePhysics` _mesh true)
      (`PrimitiveComponent.AddImpulse` _mesh (0.0 0.0 3000.0) "None" true))))

(event `self.CollisionBox.OnComponentEndOverlap`
  (params (OverlappedComponent :type "PrimitiveComponent Object Reference") (OtherActor :type "Actor Object Reference") (OtherComp :type "PrimitiveComponent Object Reference") (OtherBodyIndex :type Integer))
  (bind _asbp_player_character (cast `/Game/GameFiles/Characters/BP_PlayerCharacter` OtherActor))
  (set `CharacterMovementComponent.JumpZVelocity` 300.0 (`Character.CharacterMovement` _asbp_player_character)))

(fn `UserConstructionScript`)