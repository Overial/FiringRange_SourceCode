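; Catapult actor that loads the player as its payload and releases them as a ragdoll, in two uses.
; The first use plays a crouch montage, disables player collision, attaches the capsule to Payload, then slowly rotates PullArm back to arm it.
; The next use snaps the arm back, detaches the player and enables mesh physics simulation.
; No explicit launch impulse is applied.
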(event `/Game/GameFiles/CatapultSystem/Blueprints/BPI_Use.FnUse`
  (bind _pullarm (`self.PullArm`))
  (bind _relativelocation (`SceneComponent.RelativeLocation` _pullarm))
  (if (`self.IsReadyToFire?`)
    (`KismetSystemLibrary.MoveComponentTo` _pullarm _relativelocation (struct) true true 0.1)
    (bind _capsulecomponent (`Character.CapsuleComponent` (stale _asbp_player_character_2)))
    (`SceneComponent.K2_DetachFromComponent` _capsulecomponent "KeepWorld" "KeepWorld" "KeepWorld" true)
    (set `self.IsReadyToFire?` false)
    (bind _asbp_player_character (cast `/Game/GameFiles/Characters/BP_PlayerCharacter` (`GameplayStatics.GetPlayerCharacter` 0)))
    (set `/Game/GameFiles/Characters/BP_PlayerCharacter.IsInRagdoll?` true _asbp_player_character)
    (bind _mesh (`Character.Mesh` _asbp_player_character))
    (`PrimitiveComponent.SetCollisionEnabled` _mesh "QueryAndPhysics")
    (`SkeletalMeshComponent.SetAllBodiesSimulatePhysics` _mesh true)
    (`PrimitiveComponent.SetSimulatePhysics` _mesh true)
    (else
      (bind _asbp_player_character_2 (cast `/Game/GameFiles/Characters/BP_PlayerCharacter` (`GameplayStatics.GetPlayerCharacter` 0)))
      (`Character.PlayAnimMontage` _asbp_player_character_2 "/Game/GameFiles/Animations/PlayerCharacter/AM_Crouch_Idle_Rifle_Hip.AM_Crouch_Idle_Rifle_Hip" 1.0 "None")
      (`PrimitiveComponent.SetCollisionEnabled` _capsulecomponent "NoCollision")
      (`PrimitiveComponent.SetCollisionEnabled` (`Character.Mesh` _asbp_player_character_2) "NoCollision")
      (`SceneComponent.K2_AttachToComponent` _capsulecomponent (`self.Payload`) "None" "SnapToTarget" "SnapToTarget" "KeepWorld" false)
      (`KismetSystemLibrary.Delay` 0.5)
      (`KismetSystemLibrary.MoveComponentTo` _pullarm _relativelocation (struct :`Pitch` 90.0) true true 2.0)
      (set `self.IsReadyToFire?` true))))

(event `self.ReceiveBeginPlay`)

(fn `UserConstructionScript`)