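; Enemy character that registers with the game mode's enemy count, gets a random walk speed, and reports sight of the player to its Blackboard through AI perception.
; Damage plays a random hit montage and pauses movement.
; At zero health it decrements the enemy count, credits the player's kill, plays a death montage, then ragdolls and may drop an ammo crate at a downward-traced point.
; The older AIMoveTo chase logic is disconnected.
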(event `self.ReceiveBeginPlay`
  (`|ExecutionSequence`
    (:`then_0`
      (bind _asbp_player_character (cast `/Game/GameFiles/Characters/BP_PlayerCharacter` (`GameplayStatics.GetPlayerCharacter` 0)))
      (set `self.PlayerRef` _asbp_player_character)
      (set `CharacterMovementComponent.MaxWalkSpeed` (select `int` (`KismetMathLibrary.RandomInteger` 2) :`0` 200.0 :`1` 250.0 :`2` 300.0 :!type "Float (single-precision)") (`self.CharacterMovement`)))
    (:`then_1`
      (bind _asthird_person_game_mode (cast `/Game/ThirdPersonBP/Blueprints/ThirdPersonGameMode` (`GameplayStatics.GetGameMode`)))
      (set `self.GameModeRef` _asthird_person_game_mode))
    (:`then_2`
      (`/Game/ThirdPersonBP/Blueprints/ThirdPersonGameMode.OnIncreaseEnemyCount` (`self.GameModeRef`)))))

(event `OnChasePlayer`
  (params (PlayerToChase :type "/Game/GameFiles/Characters/BP_PlayerCharacter Object Reference")))

(event `self.ReceiveAnyDamage`
  (params (Damage :type "Float (single-precision)") (DamageType :type "DamageType Object Reference") (InstigatedBy :type "Controller Object Reference") (DamageCauser :type "Actor Object Reference"))
  (bind _returnvalue (`self.K2_GetActorLocation`))
  (bind _returnvalue_2 (`self.K2_GetActorLocation`))
  (bind _mesh (`self.Mesh`))
  (if (not (`self.IsDead?`))
    (bind _output_get (set `self.Health` (`KismetMathLibrary.FClamp` (- (`self.Health`) Damage) 0.0 100.0)))
    (if (<= _output_get 0.0)
      (set `self.IsDead?` true)
      (`GameplayStatics.PlaySoundAtLocation` "/Game/GameFiles/Sounds/Death/A_Death_Cue.A_Death_Cue" _returnvalue (struct) 1.0 1.0 0.0 null null null)
      (`CharacterMovementComponent.DisableMovement` (`self.CharacterMovement`))
      (`/Game/ThirdPersonBP/Blueprints/ThirdPersonGameMode.OnDecreaseEnemyCount` (`self.GameModeRef`))
      (bind _returnvalue_3 (`self.PlayAnimMontage` (select `int` (`KismetMathLibrary.RandomInteger` 3) :`0` "/Game/GameFiles/Animations/Enemy/AM_Death_01.AM_Death_01" :`1` "/Game/GameFiles/Animations/Enemy/AM_Death_02.AM_Death_02" :`2` "/Game/GameFiles/Animations/Enemy/AM_Death_03.AM_Death_03" :`3` "/Game/GameFiles/Animations/Enemy/AM_Death_04.AM_Death_04" :!type "AnimMontage Object Reference")))
      (`/Engine/EditorBlueprintResources/StandardMacros.IncrementInt` (`/Game/GameFiles/Characters/BP_PlayerCharacter.KillCount` (`self.PlayerRef`))
        (:`  `
          (`KismetSystemLibrary.Delay` _returnvalue_3)
          (`PrimitiveComponent.SetCollisionEnabled` (`self.CapsuleComponent`) "NoCollision")
          (`PrimitiveComponent.SetCollisionEnabled` _mesh "QueryAndPhysics")
          (`SkeletalMeshComponent.SetAllBodiesSimulatePhysics` _mesh true)
          (`PrimitiveComponent.SetSimulatePhysics` _mesh true)
          (if (`KismetMathLibrary.RandomBoolWithWeight` 0.5)
            (bind _outhit (`KismetSystemLibrary.LineTraceSingle` _returnvalue_2 (+ _returnvalue_2 (0.0 0.0 -1500.0)) "TraceTypeQuery1"))
            (`|SpawnActorFromClass` "/Game/GameFiles/Blueprints/BP_AmmoCrate.BP_AmmoCrate_C" (`KismetMathLibrary.MakeTransform` (`.Location` (`GameplayStatics.BreakHitResult` _outhit))) "Undefined" "OverrideRootScale" null null))))
      (else
        (`GameplayStatics.PlaySoundAtLocation` "/Game/GameFiles/Sounds/Damage/A_Damage_Cue.A_Damage_Cue" _returnvalue (struct) 1.0 1.0 0.0 null null null)
        (`CharacterMovementComponent.DisableMovement` (`self.CharacterMovement`))
        (bind _returnvalue_4 (`self.PlayAnimMontage` (select `int` (`KismetMathLibrary.RandomInteger` 3) :`0` "/Game/GameFiles/Animations/Enemy/AM_Hit_01.AM_Hit_01" :`1` "/Game/GameFiles/Animations/Enemy/AM_Hit_02.AM_Hit_02" :`2` "/Game/GameFiles/Animations/Enemy/AM_Hit_03.AM_Hit_03" :`3` "/Game/GameFiles/Animations/Enemy/AM_Hit_04.AM_Hit_04" :!type "AnimMontage Object Reference")))
        (`KismetSystemLibrary.Delay` _returnvalue_4)
        (if (not (`self.IsDead?`))
          (`CharacterMovementComponent.SetMovementMode` (`self.CharacterMovement`) "MOVE_Walking" 0))))))

(event `self.AIPerception.OnTargetPerceptionUpdated`
  (params (Actor :type "Actor Object Reference") (Stimulus :type "AIStimulus Structure"))
  (cast `/Game/GameFiles/Characters/BP_PlayerCharacter` Actor)
  (`BlackboardComponent.SetValueAsBool` (`AIBlueprintHelperLibrary.GetBlackboard` null) "CanSeePlayer?" Stimulus_bSuccessfullySensed))

(fn `UserConstructionScript`)